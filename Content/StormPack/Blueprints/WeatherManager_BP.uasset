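; Weather manager Blueprint that is built to switch a referenced BP_WeatherTool randomly between rain, snow and neither.
; FChangeWeather uses a looping random MultiGate to set the tool's rain and snow flags.
; Tick sets a looping timer for it with a random whole-minute delay.
; Because this runs every frame, the timer keeps restarting before it can fire.
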(event `self.ReceiveTick`
  (params (DeltaSeconds :type "Float (single-precision)"))
  (`KismetSystemLibrary.K2_SetTimer` null "FChangeWeather" (* (`KismetMathLibrary.Conv_IntToDouble` (+ (`KismetMathLibrary.RandomInteger` 4) 1)) 60.0) true))

(event `self.ReceiveBeginPlay`)

(fn `FChangeWeather`
  (bind _weathertool (`self.weatherTool`))
  (`|MultiGate` true true
    (:`Out 0`
      (bind _asbp_weather_tool (cast `/Game/StormPack/Blueprints/BP_WeatherTool` _weathertool))
      (set `/Game/StormPack/Blueprints/BP_WeatherTool.Enable Rain` true _asbp_weather_tool)
      (set `/Game/StormPack/Blueprints/BP_WeatherTool.Enable Snow` false _asbp_weather_tool))
    (:`Out 1`
      (bind _asbp_weather_tool_2 (cast `/Game/StormPack/Blueprints/BP_WeatherTool` _weathertool))
      (set `/Game/StormPack/Blueprints/BP_WeatherTool.Enable Rain` false _asbp_weather_tool_2)
      (set `/Game/StormPack/Blueprints/BP_WeatherTool.Enable Snow` true _asbp_weather_tool_2))
    (:`Out 2`
      (bind _asbp_weather_tool_3 (cast `/Game/StormPack/Blueprints/BP_WeatherTool` _weathertool))
      (set `/Game/StormPack/Blueprints/BP_WeatherTool.Enable Rain` false _asbp_weather_tool_3)
      (set `/Game/StormPack/Blueprints/BP_WeatherTool.Enable Snow` false _asbp_weather_tool_3))))

(fn `UserConstructionScript`)